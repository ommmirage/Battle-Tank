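; Player-controllable tank Blueprint that assembles its hull, turret, barrel and tracks, then handles camera aim, firing and a forward-drive input.
; Construction attaches the parts via sockets, and BeginPlay registers the barrel and turret references.
; Aim axes rotate the azimuth gimbal and spring arm, while Fire delegates to a Fire function.
; Forward applies one force per press, taken from the left track but applied at the right track's location, and prints it.
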(event `self.ReceiveBeginPlay`
  (`self.SetBarrelReference` (`self.Barrel`))
  (`self.SetTurretReference` (`self.Turret`)))

(event `InputAxis|Aim Azimuth`
  (params (AxisValue :type "Float (single-precision)"))
  ;[1 1 1] Camera rotation
  (`SceneComponent.K2_AddLocalRotation` (`self.Azmuth Gimbal`) (`KismetMathLibrary.MakeRotator` 0.0 0.0 (* AxisValue 2.0)) false false))

(event `InputAxis|Aim Elevation`
  (params (AxisValue :type "Float (single-precision)"))
  ;[1 1 1] Camera rotation
  (`SceneComponent.K2_AddLocalRotation` (`self.SpringArm`) (`KismetMathLibrary.MakeRotator` 0.0 AxisValue) false false))

(event `InputAction|Fire`
  (params (Key :type "Key Structure"))
  (:`Pressed`
    (`self.Fire`)))

(event `InputAction|Forward`
  (params (Key :type "Key Structure"))
  (:`Pressed`
    (bind _force_applied (`/Game/Blueprints/TankTrack_BP.Get Force and Location` (`self.LeftTrack_BP`)))
    (`PrimitiveComponent.AddForceAtLocation` (`self.Tank`) _force_applied (`SceneComponent.GetSocketLocation` (`self.RightTrack`) "None") "None")
    (`KismetSystemLibrary.PrintString` (`KismetStringLibrary.Conv_VectorToString` _force_applied))))

(fn `UserConstructionScript`
  (`StaticMeshComponent.SetStaticMesh` (`self.Barrel`) "/Game/Tank/tank_fbx_Barrel.tank_fbx_Barrel")
  (`StaticMeshComponent.SetStaticMesh` (`self.Turret`) "/Game/Tank/tank_fbx_Turret.tank_fbx_Turret")
  (`SceneComponent.K2_AttachToComponent` (`self.Turret`) (`self.Tank`) "Turret" "KeepRelative" "KeepRelative" "KeepRelative" true)
  (`SceneComponent.K2_AttachToComponent` (`self.Barrel`) (`self.Turret`) "Barrel" "KeepRelative" "KeepRelative" "KeepRelative" true)
  (`SceneComponent.K2_AttachToComponent` (`self.LeftTrack_BP`) (`self.Tank`) "Left Track" "KeepRelative" "KeepRelative" "KeepRelative" true)
  (`SceneComponent.K2_AttachToComponent` (`self.RightTrack`) (`self.Tank`) "Right Track" "KeepRelative" "KeepRelative" "KeepRelative" true))